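; BP_MasterItems is a base actor for items the player can hover over and pick up, with OnActorInteracted left empty as an extension hook.
; Interface hover events toggle a custom depth stencil outline on the static mesh and the interaction indicator on the player's HUD.
; Interaction fires the hook, refreshes the HUD item count, hides the indicator and destroys the actor.
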(event `/Game/ThirdPerson/Blueprints/Interface/BI_Interaction.OnHovered`
  (params (isHovered :type Boolean) (PlayerRef :type "/Game/ThirdPerson/Blueprints/BP_ThirdPersonCharacter Object Reference"))
  ;[1 1 1] Interface Event Implementation
  (`/Engine/EditorBlueprintResources/StandardMacros.IsValid` PlayerRef
    (:`Is Valid`
      (`self.ToogleOutline` isHovered)
      (`/Game/ThirdPerson/Blueprints/UI/WBP_PlayerHUD.ToogleInteractionIndicator` (`/Game/ThirdPerson/Blueprints/BP_ThirdPersonCharacter.PlayerHUD Ref` PlayerRef) isHovered))))

(event `/Game/ThirdPerson/Blueprints/Interface/BI_Interaction.OnInteracted`
  (params (`Player Ref` :type "/Game/ThirdPerson/Blueprints/BP_ThirdPersonCharacter Object Reference"))
  ;[1 1 1] Interface Event Implementation
  (`/Engine/EditorBlueprintResources/StandardMacros.IsValid` `Player Ref`
    (:`Is Valid`
      (`self.OnActorInteracted` `Player Ref`)
      (`/Game/ThirdPerson/Blueprints/UI/WBP_PlayerHUD.UpdateItemsCount` (`/Game/ThirdPerson/Blueprints/BP_ThirdPersonCharacter.PlayerHUD Ref` `Player Ref`) `Player Ref`)
      (`/Game/ThirdPerson/Blueprints/UI/WBP_PlayerHUD.ToogleInteractionIndicator` (`/Game/ThirdPerson/Blueprints/BP_ThirdPersonCharacter.PlayerHUD Ref` `Player Ref`) false)
      (`self.K2_DestroyActor`))))

(event `OnActorInteracted`
  (params (PlayerRef :type "/Game/ThirdPerson/Blueprints/BP_ThirdPersonCharacter Object Reference")))

(fn `ToogleOutline`
  (params (`isVisible?` :type Boolean))
  (bind _staticmesh (`self.StaticMesh`))
  (`PrimitiveComponent.SetRenderCustomDepth` _staticmesh `isVisible?`)
  (`PrimitiveComponent.SetCustomDepthStencilValue` _staticmesh (`KismetMathLibrary.SelectInt` 1 0 `isVisible?`)))

(fn `UserConstructionScript`)