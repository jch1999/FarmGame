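; BP_Grape is an interactable grape pickup actor that gives grapes to the player.
; When interacted with, it adds its Amount to the player's Grape count and posts an item notification with the grape icon and amount on the player's HUD.
; It does not destroy or disable itself in this graph, and its BeginPlay, overlap and Tick events are unused.
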(event `self.OnActorInteracted`
  (params (PlayerRef :type "/Game/ThirdPerson/Blueprints/BP_ThirdPersonCharacter Object Reference"))
  (bind _amount (`self.Amount`))
  (set `/Game/ThirdPerson/Blueprints/BP_ThirdPersonCharacter.Grape` (+ (`/Game/ThirdPerson/Blueprints/BP_ThirdPersonCharacter.Grape` PlayerRef) _amount) PlayerRef)
  (`/Game/ThirdPerson/Blueprints/UI/WBP_PlayerHUD.AddItemNotification` (`/Game/ThirdPerson/Blueprints/BP_ThirdPersonCharacter.PlayerHUD Ref` PlayerRef) "Grape" "/Game/3DAssets/Icon_Grape.Icon_Grape" _amount))

(fn `UserConstructionScript`
  (`parent.UserConstructionScript`))