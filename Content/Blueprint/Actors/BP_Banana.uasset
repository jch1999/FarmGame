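; BP_Banana is an interactable actor that gives the player bananas.
; On OnActorInteracted, it adds Amount to the Banana count on the passed player reference, then shows an item notification with the banana icon and amount through that player's HUD.
; The graph does not destroy or disable the actor after interaction, and its BeginPlay, overlap and Tick events are unused.
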(event `self.OnActorInteracted`
  (params (PlayerRef :type "/Game/ThirdPerson/Blueprints/BP_ThirdPersonCharacter Object Reference"))
  (set `/Game/ThirdPerson/Blueprints/BP_ThirdPersonCharacter.Banana` (+ (`/Game/ThirdPerson/Blueprints/BP_ThirdPersonCharacter.Banana` PlayerRef) (`self.Amount`)) PlayerRef)
  (`/Game/ThirdPerson/Blueprints/UI/WBP_PlayerHUD.AddItemNotification` (`/Game/ThirdPerson/Blueprints/BP_ThirdPersonCharacter.PlayerHUD Ref` PlayerRef) "Banana" "/Game/ThirdParty/3DAssets/Icon_Banana.Icon_Banana" (`self.Amount`)))

(fn `UserConstructionScript`
  (`parent.UserConstructionScript`))