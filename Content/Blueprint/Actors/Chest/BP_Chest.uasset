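; Interactable loot chest that opens once and gives the player a random bundle of fruit.
; Hovering an unopened chest highlights it through custom depth stencil and toggles the HUD interaction indicator.
; Interacting marks it opened, swings the lid with a timeline, then clears the highlight.
; Nested weighted random branches pick the items, adding to the player's counters and updating HUD notifications and counts.
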(event `/Game/ThirdPerson/Blueprints/Interface/BI_Interaction.OnInteracted`
  (params (`Player Ref` :type "/Game/ThirdPerson/Blueprints/BP_ThirdPersonCharacter Object Reference"))
  (`/Engine/EditorBlueprintResources/StandardMacros.IsValid` `Player Ref`
    (:`Is Valid`
      (if (not (`self.isOpened?`))
        (`self.OpenChest` `Player Ref`)
        (`self.AddItemsToPlayer` `Player Ref`)))))

(event `/Game/ThirdPerson/Blueprints/Interface/BI_Interaction.OnHovered`
  (params (isHovered :type Boolean) (PlayerRef :type "/Game/ThirdPerson/Blueprints/BP_ThirdPersonCharacter Object Reference"))
  (bind _chestmesh (`self.ChestMesh`))
  ;[1 1 1] On Hovered
  (if (not (`self.isOpened?`))
    (`PrimitiveComponent.SetRenderCustomDepth` _chestmesh isHovered)
    (`PrimitiveComponent.SetRenderCustomDepth` (`self.ChestTop`) isHovered)
    (`PrimitiveComponent.SetCustomDepthStencilValue` _chestmesh (`KismetMathLibrary.SelectInt` 1 0 isHovered))
    (`PrimitiveComponent.SetCustomDepthStencilValue` (`self.ChestTop`) (`KismetMathLibrary.SelectInt` 1 0 isHovered))
    (`/Game/ThirdPerson/Blueprints/UI/WBP_PlayerHUD.ToogleInteractionIndicator` (`/Game/ThirdPerson/Blueprints/BP_ThirdPersonCharacter.PlayerHUD Ref` PlayerRef) isHovered)))

(event `AddItemsToPlayer`
  (params (`Player Ref` :type "/Game/ThirdPerson/Blueprints/BP_ThirdPersonCharacter Object Reference"))
  (bind _playerhud_ref (`/Game/ThirdPerson/Blueprints/BP_ThirdPersonCharacter.PlayerHUD Ref` `Player Ref`))
  ;[1 1 1] Add Items To The Player (Randomized)
  (if (`KismetMathLibrary.RandomBoolWithWeight` 0.5)
    (set `/Game/ThirdPerson/Blueprints/BP_ThirdPersonCharacter.Apple` (+ (`/Game/ThirdPerson/Blueprints/BP_ThirdPersonCharacter.Apple` `Player Ref`) 1) `Player Ref`)
    (set `/Game/ThirdPerson/Blueprints/BP_ThirdPersonCharacter.Banana` (+ (`/Game/ThirdPerson/Blueprints/BP_ThirdPersonCharacter.Banana` `Player Ref`) 2) `Player Ref`)
    (`/Game/ThirdPerson/Blueprints/UI/WBP_PlayerHUD.AddItemNotification` _playerhud_ref "Banana" "/Game/ThirdParty/3DAssets/Icon_Banana.Icon_Banana" 2)
    (`/Game/ThirdPerson/Blueprints/UI/WBP_PlayerHUD.AddItemNotification` _playerhud_ref "Apple" "/Game/ThirdParty/3DAssets/Icon_Apple.Icon_Apple" 1)
    (elif (`KismetMathLibrary.RandomBoolWithWeight` 0.25)
      (set `/Game/ThirdPerson/Blueprints/BP_ThirdPersonCharacter.Grape` (+ (`/Game/ThirdPerson/Blueprints/BP_ThirdPersonCharacter.Grape` `Player Ref`) 2) `Player Ref`)
      (bind _output_get (set `/Game/ThirdPerson/Blueprints/BP_ThirdPersonCharacter.Apple` (+ (stale _output_get) 1) `Player Ref`))
      (`/Game/ThirdPerson/Blueprints/UI/WBP_PlayerHUD.AddItemNotification` _playerhud_ref "Apple" "/Game/ThirdParty/3DAssets/Icon_Apple.Icon_Apple" 1)
      (`/Game/ThirdPerson/Blueprints/UI/WBP_PlayerHUD.AddItemNotification` _playerhud_ref "Grape" "/Game/ThirdParty/3DAssets/Icon_Grape.Icon_Grape" 2)
      (else
        (bind _output_get_2 (set `/Game/ThirdPerson/Blueprints/BP_ThirdPersonCharacter.Banana` (+ (stale _output_get_2) 2) `Player Ref`))
        (`/Game/ThirdPerson/Blueprints/UI/WBP_PlayerHUD.AddItemNotification` _playerhud_ref "Banana" "/Game/ThirdParty/3DAssets/Icon_Banana.Icon_Banana" 2))))
  (`/Game/ThirdPerson/Blueprints/UI/WBP_PlayerHUD.UpdateItemsCount` _playerhud_ref `Player Ref`))

(event `OpenChest`
  (params (`Player Ref` :type "/Game/ThirdPerson/Blueprints/BP_ThirdPersonCharacter Object Reference"))
  (bind _chestmesh (`self.ChestMesh`))
  (bind _chesttop (`self.ChestTop`))
  (bind (_relativerotation_roll _relativerotation_pitch _relativerotation_yaw) (`KismetMathLibrary.BreakRotator` (`SceneComponent.RelativeRotation` _chesttop)))
  (set `self.isOpened?` true)
  (bind (_direction _lerp_value) (`Timeline|Timeline_OpenChest`)
    (:`Update`
      (`SceneComponent.K2_SetRelativeRotation` _chesttop (`KismetMathLibrary.MakeRotator` (`KismetMathLibrary.Lerp` 0.0 110.0 _lerp_value) _relativerotation_pitch _relativerotation_yaw) false false))
    (:`Finished`
      (`PrimitiveComponent.SetRenderCustomDepth` _chestmesh false)
      (`PrimitiveComponent.SetRenderCustomDepth` (`self.ChestTop`) false)
      (`PrimitiveComponent.SetCustomDepthStencilValue` _chestmesh 0)
      (`PrimitiveComponent.SetCustomDepthStencilValue` (`self.ChestTop`) 0)
      (`/Game/ThirdPerson/Blueprints/UI/WBP_PlayerHUD.ToogleInteractionIndicator` (`/Game/ThirdPerson/Blueprints/BP_ThirdPersonCharacter.PlayerHUD Ref` `Player Ref`) false))))

(fn `UserConstructionScript`)